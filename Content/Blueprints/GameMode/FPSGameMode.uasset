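; FPS game mode that tracks how many drones remain in the level and shows the count on screen.
; BeginPlay creates the GameModeHUD widget, counts all DronePawn actors and writes that number to the HUD's drone text.
; The DroneDied function decrements the count and refreshes the text; the only call to it in this event graph is unconnected.
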(event EventBeginPlay
  ;[0.3869 0.9 1] Add Game Mode HUD
  (bind _returnvalue (UserInterface|CreateWidget "/Game/Blueprints/HUD/GameModeHUD.GameModeHUD_C"))
  (bind _output_get (Variables|Default|SetGameModeHud _returnvalue))
  (UserInterface|Viewport|AddtoViewport _output_get 0)
  ;[0.7865 0.252 1] Set Number of Drones
  (bind _outactors (Actor|GetAllActorsOfClass "/Game/Blueprints/Drone/DronePawn.DronePawn_C"))
  (Variables|Default|SetNoOf%20Drones (Utilities|Array|Length _outactors))
  (Rendering|Components|TextRender|SetText (Variables|/Game/Blueprints/HUD/GameModeHUD.GameModeHUD_C|GetDroneText (Variables|Default|GetGameModeHud)) (Utilities|Text|ToText(Integer) (Utilities|Array|Length _outactors))))

(fn ConstructionScript)

(fn DroneDied
  (bind _result (Math|Integer|DecrementInt (Variables|Default|GetNoOf%20Drones))
    (:%20%20
      (Rendering|Components|TextRender|SetText (Variables|/Game/Blueprints/HUD/GameModeHUD.GameModeHUD_C|GetDroneText (Variables|Default|GetGameModeHud)) (Utilities|Text|ToText(Integer) _result)))))